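; BP_AIZombie is a zombie enemy that chases the player on sight and can be killed by damage.
; PawnSensing starts an AI move toward any seen PhasePlayerCharacter and sets CanSeeEnemy, which a retriggerable delay clears shortly after sightings stop.
; Any damage lowers Health, and at zero or below it plays a death sound and switches the mesh to physics simulation.
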(event OnSeePawn(PawnSensing)
  (params (Pawn :type Pawn%20Object%20Reference))
  (bind _asphase_player_character (Utilities|Casting|CastToPhasePlayerCharacter Pawn))
  (Utilities|FlowControl|Sequence
    (:then_0
      (Variables|Default|SetCanSeeEnemy true)
      (AI|AIMoveTo self "0, 0, 0" _asphase_player_character 5.0 false))
    (:then_1
      (Utilities|FlowControl|RetriggerableDelay 0.5)
      (Variables|Default|SetCanSeeEnemy false))))

(event EventBeginPlay)

(event Collision|EventActorBeginOverlap
  (params (OtherActor :type Actor%20Object%20Reference)))

(event EventTick
  (params (DeltaSeconds :type Float%20%28single-precision%29)))

(event Game|Damage|EventAnyDamage
  (params (Damage :type Float%20%28single-precision%29) (DamageType :type Damage%20Type%20Object%20Reference) (InstigatedBy :type Controller%20Object%20Reference) (DamageCauser :type Actor%20Object%20Reference))
  (bind _output_get (Variables|Default|SetHealth (- (Variables|Default|GetHealth) Damage)))
  (if (<= _output_get 0.0)
    (Audio|PlaySound2D "/Game/enemy_dead_00.enemy_dead_00" 1.0 1.0 0.0 0 0)
    (Physics|SetSimulatePhysics (Variables|Character|GetMesh) true)))

(fn ConstructionScript)